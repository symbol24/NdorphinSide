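; Player controller for the character select screen, giving each player their own selection widget.
; After a short delay on BeginPlay it caches the game mode and game instance, then adds the widget to the player screen with Game and UI input.
; Keyboard and gamepad keys send navigation requests to the widget or pick one of two characters.
; The first pick locks, registers character and controller ID in the game instance, and updates the game mode menu's player image.
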(event EventBeginPlay
  (Utilities|FlowControl|Delay 0.2)
  (bind _ascharacter_select_screen_game_mode (Utilities|Casting|CastToCharacterSelectScreenGameMode (Game|GetGameMode)))
  (Variables|Default|SetGameMode _ascharacter_select_screen_game_mode)
  (bind _asndorphin_instance (Utilities|Casting|CastToNdorphinInstance (Game|GetGameInstance)))
  (Variables|Default|SetGameInstance _asndorphin_instance)
  (Variables|Default|SetbShowMouseCursor true)
  (bind _returnvalue (UserInterface|CreateWidget "/Game/Blueprints/Widgets]/EachPlayerSelectScreen.EachPlayerSelectScreen_C" self))
  (bind _output_get (Variables|Default|SetWidget _returnvalue))
  (UserInterface|Viewport|AddtoPlayerScreen _output_get)
  (Input|SetInputModeGameandUI self (Variables|Default|GetWidget) "DoNotLock" true))

(event Input|GamepadEvents|GamepadSpecialRight
  (params (Key :type Key%20Structure))
  (:Pressed
    (Variables|Default|SetCharacterID 0)
    (if (not (Variables|Default|GetHasSelected))
      (bind _returnvalue (Class|GameplayStatics|GetPlayerControllerID self))
      (Default|CreateNewPlayerContainer (Variables|Default|GetGameInstance) (Variables|Default|GetCharacterID) _returnvalue)
      (Variables|Default|SetHasSelected true)
      (Default|UpdatePlayerImage (Variables|/Game/Blueprints/Gamemodes/CharacterSelectScreenGameMode.CharacterSelectScreenGameMode_C|GetMenuWidget (Variables|Default|GetGameMode)) (Variables|Default|GetCharacterID))
      (Class|GameplayStatics|GetPlayerControllerID self))))

(event Input|KeyboardEvents|1
  (params (Key :type Key%20Structure))
  (:Pressed
    (Variables|Default|SetCharacterID 0)
    (if (not (Variables|Default|GetHasSelected))
      (bind _returnvalue (Class|GameplayStatics|GetPlayerControllerID self))
      (Default|CreateNewPlayerContainer (Variables|Default|GetGameInstance) (Variables|Default|GetCharacterID) _returnvalue)
      (Variables|Default|SetHasSelected true)
      (Default|UpdatePlayerImage (Variables|/Game/Blueprints/Gamemodes/CharacterSelectScreenGameMode.CharacterSelectScreenGameMode_C|GetMenuWidget (Variables|Default|GetGameMode)) (Variables|Default|GetCharacterID))
      (Class|GameplayStatics|GetPlayerControllerID self))))

(event Input|GamepadEvents|GamepadFaceButtonLeft
  (params (Key :type Key%20Structure))
  (:Pressed
    (Variables|Default|SetCharacterID 1)
    (if (not (Variables|Default|GetHasSelected))
      (bind _returnvalue (Class|GameplayStatics|GetPlayerControllerID self))
      (Default|CreateNewPlayerContainer (Variables|Default|GetGameInstance) (Variables|Default|GetCharacterID) _returnvalue)
      (Variables|Default|SetHasSelected true)
      (Default|UpdatePlayerImage (Variables|/Game/Blueprints/Gamemodes/CharacterSelectScreenGameMode.CharacterSelectScreenGameMode_C|GetMenuWidget (Variables|Default|GetGameMode)) (Variables|Default|GetCharacterID))
      (Class|GameplayStatics|GetPlayerControllerID self))))

(event Input|KeyboardEvents|2
  (params (Key :type Key%20Structure))
  (:Pressed
    (Variables|Default|SetCharacterID 1)
    (if (not (Variables|Default|GetHasSelected))
      (bind _returnvalue (Class|GameplayStatics|GetPlayerControllerID self))
      (Default|CreateNewPlayerContainer (Variables|Default|GetGameInstance) (Variables|Default|GetCharacterID) _returnvalue)
      (Variables|Default|SetHasSelected true)
      (Default|UpdatePlayerImage (Variables|/Game/Blueprints/Gamemodes/CharacterSelectScreenGameMode.CharacterSelectScreenGameMode_C|GetMenuWidget (Variables|Default|GetGameMode)) (Variables|Default|GetCharacterID))
      (Class|GameplayStatics|GetPlayerControllerID self))))

(event Input|GamepadEvents|GamepadLeftShoulder
  (params (Key :type Key%20Structure))
  (:Pressed
    (Default|ReceiveNavigationRequest (Variables|Default|GetWidget) "NewEnumerator0")))

(event Input|GamepadEvents|GamepadRightShoulder
  (params (Key :type Key%20Structure))
  (:Pressed
    (Default|ReceiveNavigationRequest (Variables|Default|GetWidget) "NewEnumerator1")))

(event Input|KeyboardEvents|P
  (params (Key :type Key%20Structure))
  (:Pressed
    (Default|ReceiveNavigationRequest (Variables|Default|GetWidget) "NewEnumerator0")))

(event Input|KeyboardEvents|O
  (params (Key :type Key%20Structure))
  (:Pressed
    (Default|ReceiveNavigationRequest (Variables|Default|GetWidget) "NewEnumerator1")))

(fn ConstructionScript
  (|CallParentFunction))