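; Player controller that lets a player spawn or despawn a character through keyboard and gamepad input.
; Spawn inputs pass one of two character IDs to NewSuperGameMode, and the despawn input asks it to remove the character.
; An IsSpawned flag blocks repeat requests.
; Tick feeds a one-second Delay that prints PlayerIDCache for debugging.
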(event EventTick
  (params (DeltaSeconds :type Float%20%28single-precision%29))
  (Utilities|FlowControl|Delay 1.0)
  (Development|PrintString (Utilities|String|ToString(Integer) (Variables|Default|GetPlayerIDCache))))

(event Input|GamepadEvents|GamepadSpecialLeft
  (params (Key :type Key%20Structure))
  (:Pressed
    (if (Variables|Default|GetIsSpawned)
      (bind _asnew_super_game_mode (Utilities|Casting|CastToNewSuperGameMode (Game|GetGameMode)))
      (Default|DespawnCharacter _asnew_super_game_mode self)
      (Variables|Default|SetIsSpawned false))))

(event Input|GamepadEvents|GamepadSpecialRight
  (params (Key :type Key%20Structure))
  (:Pressed
    (if (not (Variables|Default|GetIsSpawned))
      (Variables|Default|SetID 0)
      (bind _asnew_super_game_mode (Utilities|Casting|CastToNewSuperGameMode (Game|GetGameMode)))
      (Default|SpawnCharacter _asnew_super_game_mode self (Variables|Default|GetID))
      (Variables|Default|SetIsSpawned true))))

(event Input|KeyboardEvents|1
  (params (Key :type Key%20Structure))
  (:Pressed
    (if (not (Variables|Default|GetIsSpawned))
      (Variables|Default|SetID 0)
      (bind _asnew_super_game_mode (Utilities|Casting|CastToNewSuperGameMode (Game|GetGameMode)))
      (Default|SpawnCharacter _asnew_super_game_mode self (Variables|Default|GetID))
      (Variables|Default|SetIsSpawned true))))

(event Input|GamepadEvents|GamepadFaceButtonLeft
  (params (Key :type Key%20Structure))
  (:Pressed
    (if (not (Variables|Default|GetIsSpawned))
      (Variables|Default|SetID 1)
      (bind _asnew_super_game_mode (Utilities|Casting|CastToNewSuperGameMode (Game|GetGameMode)))
      (Default|SpawnCharacter _asnew_super_game_mode self (Variables|Default|GetID))
      (Variables|Default|SetIsSpawned true))))

(event Input|KeyboardEvents|2
  (params (Key :type Key%20Structure))
  (:Pressed
    (if (not (Variables|Default|GetIsSpawned))
      (Variables|Default|SetID 1)
      (bind _asnew_super_game_mode (Utilities|Casting|CastToNewSuperGameMode (Game|GetGameMode)))
      (Default|SpawnCharacter _asnew_super_game_mode self (Variables|Default|GetID))
      (Variables|Default|SetIsSpawned true))))

(event Input|KeyboardEvents|3
  (params (Key :type Key%20Structure))
  (:Pressed
    (if (Variables|Default|GetIsSpawned)
      (bind _asnew_super_game_mode (Utilities|Casting|CastToNewSuperGameMode (Game|GetGameMode)))
      (Default|DespawnCharacter _asnew_super_game_mode self)
      (Variables|Default|SetIsSpawned false))))

(fn ConstructionScript)