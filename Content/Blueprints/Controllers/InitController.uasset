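; Player controller that lets a player spawn as one of two characters, or despawn, via keyboard or gamepad.
; An IsSpawned flag gates the input, and the SuperSideScrollingGameMode does the spawning and despawning, with despawn always passing player ID zero.
; GetPlayerContainer matches the controller ID against the NdorphinInstance's player list or registers a new entry, supplying the player and character IDs for spawning.
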(event Input|GamepadEvents|GamepadSpecialLeft
  (params (Key :type Key%20Structure))
  (:Pressed
    (if (Variables|Default|GetIsSpawned)
      (bind _assuper_side_scrolling_game_mode (Utilities|Casting|CastToSuperSideScrollingGameMode (Game|GetGameMode)))
      (Default|DespawnCharacter _assuper_side_scrolling_game_mode self)
      (Variables|Default|SetIsSpawned false))))

(event Input|GamepadEvents|GamepadSpecialRight
  (params (Key :type Key%20Structure))
  (:Pressed
    (if (not (Variables|Default|GetIsSpawned))
      (Variables|Default|SetCharacterID 0)
      (bind _assuper_side_scrolling_game_mode (Utilities|Casting|CastToSuperSideScrollingGameMode (Game|GetGameMode)))
      (bind _newplayercontainer (CallFunction|GetPlayerContainer))
      (Default|SpawnCharacter _assuper_side_scrolling_game_mode self _newplayercontainer)
      (Variables|Default|SetIsSpawned true))))

(event Input|KeyboardEvents|1
  (params (Key :type Key%20Structure))
  (:Pressed
    (if (not (Variables|Default|GetIsSpawned))
      (Variables|Default|SetCharacterID 0)
      (bind _assuper_side_scrolling_game_mode (Utilities|Casting|CastToSuperSideScrollingGameMode (Game|GetGameMode)))
      (bind _newplayercontainer (CallFunction|GetPlayerContainer))
      (Default|SpawnCharacter _assuper_side_scrolling_game_mode self _newplayercontainer)
      (Variables|Default|SetIsSpawned true))))

(event Input|GamepadEvents|GamepadFaceButtonLeft
  (params (Key :type Key%20Structure))
  (:Pressed
    (if (not (Variables|Default|GetIsSpawned))
      (Variables|Default|SetCharacterID 1)
      (bind _assuper_side_scrolling_game_mode (Utilities|Casting|CastToSuperSideScrollingGameMode (Game|GetGameMode)))
      (bind _newplayercontainer (CallFunction|GetPlayerContainer))
      (Default|SpawnCharacter _assuper_side_scrolling_game_mode self _newplayercontainer)
      (Variables|Default|SetIsSpawned true))))

(event Input|KeyboardEvents|2
  (params (Key :type Key%20Structure))
  (:Pressed
    (if (not (Variables|Default|GetIsSpawned))
      (Variables|Default|SetCharacterID 1)
      (bind _assuper_side_scrolling_game_mode (Utilities|Casting|CastToSuperSideScrollingGameMode (Game|GetGameMode)))
      (bind _newplayercontainer (CallFunction|GetPlayerContainer))
      (Default|SpawnCharacter _assuper_side_scrolling_game_mode self _newplayercontainer)
      (Variables|Default|SetIsSpawned true))))

(event Input|KeyboardEvents|3
  (params (Key :type Key%20Structure))
  (:Pressed
    (if (Variables|Default|GetIsSpawned)
      (bind _assuper_side_scrolling_game_mode (Utilities|Casting|CastToSuperSideScrollingGameMode (Game|GetGameMode)))
      (Default|DespawnCharacter _assuper_side_scrolling_game_mode self)
      (Variables|Default|SetIsSpawned false))))

(fn ConstructionScript)

(fn GetPlayerContainer
  (bind _asndorphin_instance (Utilities|Casting|CastToNdorphinInstance (Game|GetGameInstance)))
  (bind _returnvalue (Class|GameplayStatics|GetPlayerControllerID self))
  (for _array_element (Variables|/Game/Blueprints/NdorphinInstance.NdorphinInstance_C|GetPlayerContainers _asndorphin_instance)
    (if (== _returnvalue (Utilities|Struct|BreakPlayerContainer _array_element))
      (bind _structout (Utilities|Struct|SetmembersinPlayerContainer _array_element (Variables|Default|GetCharacterID)))
      (LocalVariables|SetPlayerContainer _structout)
      (LocalVariables|SetIsAlreadyListed true)))
  (if (LocalVariables|GetIsAlreadyListed)
    (Development|PrintText (Utilities|Text|ToText(Integer) (Utilities|Struct|BreakPlayerContainer (LocalVariables|GetPlayerContainer))))
    (else
      (bind _returnvalue_2 (Class|GameplayStatics|GetPlayerControllerID self))
      (bind _structout_2 (Utilities|Struct|SetmembersinPlayerContainer (LocalVariables|GetPlayerContainer) (Utilities|Array|Length (Variables|/Game/Blueprints/NdorphinInstance.NdorphinInstance_C|GetPlayerContainers _asndorphin_instance)) (Variables|Default|GetCharacterID) _returnvalue_2))
      (Utilities|Array|Add (Variables|/Game/Blueprints/NdorphinInstance.NdorphinInstance_C|GetPlayerContainers _asndorphin_instance) _structout_2)))
  (return (LocalVariables|GetPlayerContainer)))