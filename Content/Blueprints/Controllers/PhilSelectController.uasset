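; Player controller for a character selection screen, translating gamepad and keyboard input into per-player selection requests.
; A three-state machine (inactive, selecting, confirmed) decides whether input activates the player, cycles characters, confirms, backs out or loads the level.
; Helper functions update the state and forward each action to PhilSelectGameMode, tagged with the controller ID except for level loading.
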(event EventBeginPlay
  (bind _asphil_select_game_mode (Utilities|Casting|CastToPhilSelectGameMode (Game|GetGameMode)))
  (Variables|Default|SetGameMode _asphil_select_game_mode))

(event Input|KeyboardEvents|Enter
  (params (Key :type Key%20Structure))
  ;[1 1 1] Start / A button / Enter / SpaceBar  ---- Start Activatin, confirm selection, load level
  (:Pressed
    (switch Utilities|FlowControl|Switch|SwitchonCharacterSelectState (Variables|Default|GetState)
      (:NewEnumerator0
        (CallFunction|SendActivationEvent))
      (:NewEnumerator1
        (CallFunction|SendConfirmEvent))
      (:NewEnumerator2
        (CallFunction|SendLoadLevelEvent)))))

(event Input|GamepadEvents|GamepadDPadLeft
  (params (Key :type Key%20Structure))
  ;[1 1 1] D-pad Left / A key / <- --- Move selection left
  (:Pressed
    (switch Utilities|FlowControl|Switch|SwitchonCharacterSelectState (Variables|Default|GetState)
      (:NewEnumerator1
        (CallFunction|SendCharacterChangeEvent false)))))

(event Input|KeyboardEvents|A
  (params (Key :type Key%20Structure))
  ;[1 1 1] D-pad Left / A key / <- --- Move selection left
  (:Pressed
    (switch Utilities|FlowControl|Switch|SwitchonCharacterSelectState (Variables|Default|GetState)
      (:NewEnumerator1
        (CallFunction|SendCharacterChangeEvent false)))))

(event Input|KeyboardEvents|Left
  (params (Key :type Key%20Structure))
  ;[1 1 1] D-pad Left / A key / <- --- Move selection left
  (:Pressed
    (switch Utilities|FlowControl|Switch|SwitchonCharacterSelectState (Variables|Default|GetState)
      (:NewEnumerator1
        (CallFunction|SendCharacterChangeEvent false)))))

(event Input|GamepadEvents|GamepadFaceButtonRight
  (params (Key :type Key%20Structure))
  ;[1 1 1] B button / Backspace --- Back out selection / Deactivate player.
  (:Pressed
    (switch Utilities|FlowControl|Switch|SwitchonCharacterSelectState (Variables|Default|GetState)
      (:NewEnumerator1
        _)
      (:NewEnumerator2
        _))
    (CallFunction|SendBackEvents)))

(event Input|GamepadEvents|GamepadDPadRight
  (params (Key :type Key%20Structure))
  ;[1 1 1] D-pad Right / D key / -> --- Move selection right
  (:Pressed
    (switch Utilities|FlowControl|Switch|SwitchonCharacterSelectState (Variables|Default|GetState)
      (:NewEnumerator1
        (CallFunction|SendCharacterChangeEvent true)))))

(event Input|KeyboardEvents|D
  (params (Key :type Key%20Structure))
  ;[1 1 1] D-pad Right / D key / -> --- Move selection right
  (:Pressed
    (switch Utilities|FlowControl|Switch|SwitchonCharacterSelectState (Variables|Default|GetState)
      (:NewEnumerator1
        (CallFunction|SendCharacterChangeEvent true)))))

(event Input|KeyboardEvents|Right
  (params (Key :type Key%20Structure))
  ;[1 1 1] D-pad Right / D key / -> --- Move selection right
  (:Pressed
    (switch Utilities|FlowControl|Switch|SwitchonCharacterSelectState (Variables|Default|GetState)
      (:NewEnumerator1
        (CallFunction|SendCharacterChangeEvent true)))))

(event Input|GamepadEvents|GamepadSpecialRight
  (params (Key :type Key%20Structure))
  ;[1 1 1] Start / A button / Enter / SpaceBar  ---- Start Activatin, confirm selection, load level
  (:Pressed
    (switch Utilities|FlowControl|Switch|SwitchonCharacterSelectState (Variables|Default|GetState)
      (:NewEnumerator0
        (CallFunction|SendActivationEvent))
      (:NewEnumerator1
        (CallFunction|SendConfirmEvent))
      (:NewEnumerator2
        (CallFunction|SendLoadLevelEvent)))))

(event Input|KeyboardEvents|SpaceBar
  (params (Key :type Key%20Structure))
  ;[1 1 1] Start / A button / Enter / SpaceBar  ---- Start Activatin, confirm selection, load level
  (:Pressed
    (switch Utilities|FlowControl|Switch|SwitchonCharacterSelectState (Variables|Default|GetState)
      (:NewEnumerator0
        (CallFunction|SendActivationEvent))
      (:NewEnumerator1
        (CallFunction|SendConfirmEvent))
      (:NewEnumerator2
        (CallFunction|SendLoadLevelEvent)))))

(event Input|GamepadEvents|GamepadFaceButtonBottom
  (params (Key :type Key%20Structure))
  ;[1 1 1] Start / A button / Enter / SpaceBar  ---- Start Activatin, confirm selection, load level
  (:Pressed
    (switch Utilities|FlowControl|Switch|SwitchonCharacterSelectState (Variables|Default|GetState)
      (:NewEnumerator0
        (CallFunction|SendActivationEvent))
      (:NewEnumerator1
        (CallFunction|SendConfirmEvent))
      (:NewEnumerator2
        (CallFunction|SendLoadLevelEvent)))))

(event Input|KeyboardEvents|Backspace
  (params (Key :type Key%20Structure))
  ;[1 1 1] B button / Backspace --- Back out selection / Deactivate player.
  (:Pressed
    (switch Utilities|FlowControl|Switch|SwitchonCharacterSelectState (Variables|Default|GetState)
      (:NewEnumerator1
        _)
      (:NewEnumerator2
        _))
    (CallFunction|SendBackEvents)))

(fn ConstructionScript)

(fn SendCharacterChangeEvent
  (params (IsRight :type Boolean))
  (bind _returnvalue (Class|GameplayStatics|GetPlayerControllerID self))
  (Default|ChangeCharacterEvent (Variables|Default|GetGameMode) _returnvalue IsRight true))

(fn SendActivationEvent
  (bind _returnvalue (Class|GameplayStatics|GetPlayerControllerID self))
  (Default|ActivatePlayerEvent (Variables|Default|GetGameMode) _returnvalue)
  (Variables|Default|SetState "NewEnumerator1"))

(fn SendConfirmEvent
  (bind _returnvalue (Class|GameplayStatics|GetPlayerControllerID self))
  (Variables|Default|SetState "NewEnumerator2")
  (Default|ConfirmSelectionEvent (Variables|Default|GetGameMode) _returnvalue))

(fn SendBackEvents
  (bind _returnvalue (Class|GameplayStatics|GetPlayerControllerID self))
  (switch Utilities|FlowControl|Switch|SwitchonCharacterSelectState (Variables|Default|GetState)
    (:NewEnumerator1
      (Variables|Default|SetState "NewEnumerator0")
      (Default|BackEvent (Variables|Default|GetGameMode) _returnvalue "NewEnumerator1"))
    (:NewEnumerator2
      (Variables|Default|SetState "NewEnumerator1")
      (Default|BackEvent (Variables|Default|GetGameMode) _returnvalue "NewEnumerator2"))))

(fn SendLoadLevelEvent
  (Default|LoadLevel (Variables|Default|GetGameMode)))