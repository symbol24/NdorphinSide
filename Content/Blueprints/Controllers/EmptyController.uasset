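; EmptyController is a player controller for the side-scroller that caches its controller ID shortly after BeginPlay.
; TimeToDie passes the given player ID to SuperSideScrollingGameMode for scoring, requests a despawn with respawn, and clears IsSpawned.
; A likely temporary JumpDown input makes the character's capsule ignore WorldDynamic after a delay, without restoring it here.
; A gamepad key prints the controller ID for debugging.
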(event Custom|TimeToDie
  (params (PlayerID :type Integer))
  ;[1 1 1] Check To see who Hit Who
  (bind _assuper_side_scrolling_game_mode (Utilities|Casting|CastToSuperSideScrollingGameMode (Game|GetGameMode)))
  (Default|UpdateScorefromPlayerIdEvent _assuper_side_scrolling_game_mode PlayerID)
  (Default|DespawnCharacter _assuper_side_scrolling_game_mode self true)
  (Variables|Default|SetIsSpawned false))

(event EventBeginPlay
  (Utilities|FlowControl|Delay 0.2)
  (bind _returnvalue (Class|GameplayStatics|GetPlayerControllerID self))
  (Variables|Default|SetControllerID _returnvalue))

(event EventTick
  (params (DeltaSeconds :type Float%20%28single-precision%29)))

(event Input|ActionEvents|InputActionJumpDown
  (params (Key :type Key%20Structure))
  ;[1 1 1] JumpDown From Platform - WILL PROBABLY DELETE
  (:Pressed
    (bind _asside_scroller_character (Utilities|Casting|CastToSideScrollerCharacter (Game|GetPlayerCharacter (Variables|Default|GetControllerID))))
    (Utilities|FlowControl|Delay 0.2)
    (Collision|SetCollisionResponsetoChannel (Variables|/Script/Engine.Character|GetCapsuleComponent _asside_scroller_character) "ECC_WorldDynamic" "ECR_Ignore")))

(event Input|GamepadEvents|GamepadSpecialLeft
  (params (Key :type Key%20Structure))
  (:Pressed
    (bind _returnvalue (Class|GameplayStatics|GetPlayerControllerID self))
    (Development|PrintString (Utilities|String|ToString(Integer) _returnvalue))))

(fn ConstructionScript)