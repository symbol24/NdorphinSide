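; SelfKillController is a controller Blueprint that lets a player kill their own character and respawn in a side-scrolling game.
; Pressing 3 or the gamepad Special Left button, while IsSpawned is true, asks SuperSideScrollingGameMode to despawn the character with respawn enabled.
; It then clears IsSpawned, blocking repeat requests; nothing in this graph sets the flag back to true.
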(event EventBeginPlay
  (|CallParentFunction) ; This node is disabled and will not be called.\nDrag off pins to build functionality.
)

(event EventTick
  (params (DeltaSeconds :type Float%20%28single-precision%29))
  (|CallParentFunction DeltaSeconds) ; This node is disabled and will not be called.\nDrag off pins to build functionality.
)

(event Input|GamepadEvents|GamepadSpecialLeft
  (params (Key :type Key%20Structure))
  (:Pressed
    (if (Variables|Default|GetIsSpawned)
      (bind _assuper_side_scrolling_game_mode (Utilities|Casting|CastToSuperSideScrollingGameMode (Game|GetGameMode)))
      (Default|DespawnCharacter _assuper_side_scrolling_game_mode self true)
      (Variables|Default|SetIsSpawned false))))

(event Input|KeyboardEvents|3
  (params (Key :type Key%20Structure))
  (:Pressed
    (if (Variables|Default|GetIsSpawned)
      (bind _assuper_side_scrolling_game_mode (Utilities|Casting|CastToSuperSideScrollingGameMode (Game|GetGameMode)))
      (Default|DespawnCharacter _assuper_side_scrolling_game_mode self true)
      (Variables|Default|SetIsSpawned false))))

(fn ConstructionScript
  (|CallParentFunction))