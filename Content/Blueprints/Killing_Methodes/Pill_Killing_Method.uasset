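; Killing method component that gives its owning character a bat swing attack with a short-lived damage window.
; On BeginPlay it finds the owner's tagged bat mesh, capsule collider and target arrow, and caches the owner's controller ID and swing poses.
; Using it snaps the bat to the arrow's pose and enables pawn overlap briefly, then resets both.
; A separate event applies damage to target characters, crediting the owner as killer.
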(event EventBeginPlay
  (|CallParentFunction)
  (CallFunction|GetBat)
  (Collision|SetCollisionResponsetoChannel (Variables|Default|GetDamageCollider) "ECC_Pawn" "ECR_Ignore"))

(event EventTick
  (params (DeltaSeconds :type Float%20%28single-precision%29))
  (|CallParentFunction DeltaSeconds) ; This node is disabled and will not be called.\nDrag off pins to build functionality.
)

(event EventUseKillingMethode
  (if (Variables|Default|GetCanUse)
    (Variables|Default|SetCanUse false)
    (Development|PrintString "Pill Killing Methode")
    (Collision|SetCollisionResponsetoChannel (Variables|Default|GetDamageCollider) "ECC_Pawn" "ECR_Overlap")
    (Transformation|SetRelativeLocationAndRotation (Variables|Default|GetBat) (Variables|Default|GetTargetPosition) (Variables|Default|GetTargetRot) false false)
    (Utilities|FlowControl|Delay 0.5)
    (Collision|SetCollisionResponsetoChannel (Variables|Default|GetDamageCollider) "ECC_Pawn" "ECR_Ignore")
    (Transformation|SetRelativeLocationAndRotation (Variables|Default|GetBat) (Variables|Default|GetOriginalPos) (Variables|Default|GetOrigRot) false false)
    (Variables|Default|SetCanUse true)))

(event EventApplyDamagetoTarget
  (params (TargetToDamage :type Object%20Object%20Reference))
  (bind _asndorphin_character_parent (Utilities|Casting|CastToNdorphinCharacter_Parent TargetToDamage))
  (Default|ApplyDamageEvent _asndorphin_character_parent (Variables|Default|GetDamage) (Variables|Default|GetOwnerID)))

(fn GetBat
  (bind _returnvalue (Components|GetOwner))
  (bind _returnvalue_2 (Actor|GetComponentsbyTag _returnvalue "/Script/Engine.ArrowComponent" "Target"))
  (bind _output (Utilities|Array|Get(acopy) _returnvalue_2))
  (Utilities|FlowControl|Sequence
    (:then_0
      (if (> (Utilities|Array|Length (Actor|GetComponentsbyTag (Components|GetOwner) "/Script/Engine.StaticMeshComponent" "Bat")) 0)
        (Variables|Default|SetBat (Utilities|Array|Get(acopy) (Actor|GetComponentsbyTag (Components|GetOwner) "/Script/Engine.StaticMeshComponent" "Bat")))
        (else
          (Development|PrintText (Utilities|Text|FormatText (Utilities|Text|ToText(String) (Utilities|GetDisplayName (Components|GetOwner))) "Bat not present on {self}")))))
    (:then_1
      (if (> (Utilities|Array|Length (Actor|GetComponentsbyTag (Components|GetOwner) "/Script/Engine.CapsuleComponent" "DamageCollider")) 0)
        (Variables|Default|SetDamageCollider (Utilities|Array|Get(acopy) (Actor|GetComponentsbyTag (Components|GetOwner) "/Script/Engine.CapsuleComponent" "DamageCollider")))
        (else
          (Development|PrintText (Utilities|Text|FormatText (Utilities|Text|ToText(String) (Utilities|GetDisplayName (Components|GetOwner))) "DamageCollider not present on {self}")))))
    (:then_2
      (bind _asndorphin_character_parent (Utilities|Casting|CastToNdorphinCharacter_Parent (Components|GetOwner)))
      (bind _asempty_controller (Utilities|Casting|CastToEmptyController (Pawn|GetController _asndorphin_character_parent)))
      (bind _returnvalue_3 (Class|GameplayStatics|GetPlayerControllerID _asempty_controller))
      (Variables|Default|SetOwnerID _returnvalue_3))
    (:then_3
      (Variables|Default|SetOriginalPos (Variables|/Script/Engine.SceneComponent|GetRelativeLocation (Variables|Default|GetBat)))
      (Variables|Default|SetOrigRot (Variables|/Script/Engine.SceneComponent|GetRelativeRotation (Variables|Default|GetBat))))
    (:then_4
      (if (> (Utilities|Array|Length _returnvalue_2) 0)
        (Variables|Default|SetTargetPosition (Variables|/Script/Engine.SceneComponent|GetRelativeLocation _output))
        (Variables|Default|SetTargetRot (Variables|/Script/Engine.SceneComponent|GetRelativeRotation _output))
        (else
          (Development|PrintText (Utilities|Text|FormatText (Utilities|Text|ToText(String) (Utilities|GetDisplayName (Components|GetOwner))) "Target arrow not present on {self}")))))))

(fn SwitchDamageCollider
  (if (Utilities|Enum|Equal(Enum) (Collision|GetCollisionResponsetoChannel (Variables|Default|GetDamageCollider) "ECC_Pawn") "ECR_Ignore")
    (Collision|SetCollisionResponsetoChannel (Variables|Default|GetDamageCollider) "ECC_Pawn" "ECR_Overlap")
    (Collision|SetCollisionResponsetoChannel (Variables|Default|GetDamageCollider) "ECC_GameTraceChannel2" "ECR_Overlap")
    (else
      (Collision|SetCollisionResponsetoChannel (Variables|Default|GetDamageCollider) "ECC_Pawn" "ECR_Ignore")
      (Collision|SetCollisionResponsetoChannel (Variables|Default|GetDamageCollider) "ECC_Pawn" "ECR_Ignore"))))