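; Game mode for local multiplayer that creates extra players at BeginPlay based on the player count and caches their IDs on their controllers.
; Spawn and despawn events swap each controller's existing pawn between ShooterGuy and InitPawn at PlayerStart transforms.
; GetSpawnPoint rolls random starts, requiring an unused, enemy-free one for spawns and clearing the used flag for despawns.
; The returned transform comes from a separate random roll, so it can differ from the checked start.
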(event Custom|SpawnCharacter
  (params (PlayerController :type Player%20Controller%20Object%20Reference) (ID :type Integer))
  (bind _returnvalue (Pawn|GetControlledPawn PlayerController))
  ;[0 1 0.1363] Spawn Character
  (Utilities|IsValid _returnvalue
    (:Is%20Valid
      (Actor|DestroyActor _returnvalue)
      (bind _spawnpoint (CallFunction|GetSpawnPoint true))
      (bind _returnvalue_2 (Game|SpawnActorfromClass "/Game/Blueprints/Characters/ShooterGuy.ShooterGuy_C" _spawnpoint "Undefined" 0 0))
      (Pawn|Possess PlayerController _returnvalue_2))))

(event Custom|DespawnCharacter
  (params (PlayerController :type Player%20Controller%20Object%20Reference))
  (bind _returnvalue (Pawn|GetControlledPawn PlayerController))
  ;[1 0.08645 0.1282] DeSpawn Character
  (Utilities|IsValid _returnvalue
    (:Is%20Valid
      (Actor|DestroyActor _returnvalue)
      (bind _spawnpoint (CallFunction|GetSpawnPoint false))
      (bind _returnvalue_2 (Game|SpawnActorfromClass "/Game/Blueprints/InitPawn.InitPawn_C" _spawnpoint "Undefined" 0 0))
      (Pawn|Possess PlayerController _returnvalue_2))))

(event EventBeginPlay
  ;[1 1 1] BeginPlay Set up
  (bind _outactors (Actor|GetAllActorsOfClass "/Script/Engine.PlayerStart"))
  (Variables|Default|SetSpawnPoints _outactors)
  ;[1 1 1] CreatingPlayers
  (Utilities|FlowControl|Sequence
    (:then_0
      (switch Utilities|FlowControl|Switch|SwitchonE_NumberOfPlayers (Variables|Default|GetNumberOfPlayersInGame)
        (:NewEnumerator1
          (goto _label Reset))
        (:NewEnumerator2
          (Utilities|FlowControl|Sequence
            (:then_0
              (goto _label Reset))
            (:then_1
              (goto _label_2 Reset))))))
    (:then_1
      (bind _returnvalue (Class|GameplayStatics|CreatePlayer 1))
      (bind _asnew_player_controller (Utilities|Casting|CastToNewPlayerController _returnvalue))
      (Variables|/Game/Blueprints/Controllers/NewPlayerController.NewPlayerController_C|SetPlayerIDCache _asnew_player_controller 1)
      (Utilities|FlowControl|DoOnce true :!label _label
        (:Completed
          (bind _returnvalue_2 (Class|GameplayStatics|CreatePlayer 2))
          (bind _asnew_player_controller_2 (Utilities|Casting|CastToNewPlayerController _returnvalue_2))
          (Variables|/Game/Blueprints/Controllers/NewPlayerController.NewPlayerController_C|SetPlayerIDCache _asnew_player_controller_2 2)
          (Utilities|FlowControl|DoOnce true :!label _label_2
            (:Completed
              (bind _returnvalue_3 (Class|GameplayStatics|CreatePlayer 3))
              (bind _asnew_player_controller_3 (Utilities|Casting|CastToNewPlayerController _returnvalue_3))
              (Variables|/Game/Blueprints/Controllers/NewPlayerController.NewPlayerController_C|SetPlayerIDCache _asnew_player_controller_3 3))))))))

(fn ConstructionScript)

(fn GetCharactertoSpawn
  (params (ID :type Integer))
  (return (Utilities|Array|Get(acopy) (Variables|Default|GetCharacters) ID)))

(fn GetSpawnPoint
  (params (IsForSpawn :type Boolean))
  (bind _spawnpoints (Variables|Default|GetSpawnPoints))
  (bind _returnvalue (Utilities|Array|Length _spawnpoints))
  (bind _returnvalue_2 (- _returnvalue 1))
  (bind _returnvalue_3 (Math|Random|RandomIntegerinRange 0 _returnvalue_2))
  (bind _output (Utilities|Array|Get(acopy) _spawnpoints _returnvalue_3))
  (while (LocalVariables|GetNotFound)
    (bind _asplayer_start_ndorphin (Utilities|Casting|CastToPlayerStart_Ndorphin _output))
    (if IsForSpawn
      (if (not (or (Variables|/Game/Blueprints/PlayerStart_Ndorphin.PlayerStart_Ndorphin_C|GetEnemyClose _asplayer_start_ndorphin) (Variables|/Game/Blueprints/PlayerStart_Ndorphin.PlayerStart_Ndorphin_C|GetWasUsed _asplayer_start_ndorphin)))
        (LocalVariables|SetNotFound false)
        (Variables|/Game/Blueprints/PlayerStart_Ndorphin.PlayerStart_Ndorphin_C|SetWasUsed _asplayer_start_ndorphin true)
        (LocalVariables|SetSpawnToReturn (Transformation|GetActorTransform _output) :!label _label))
      (else
        (LocalVariables|SetNotFound false)
        (Variables|/Game/Blueprints/PlayerStart_Ndorphin.PlayerStart_Ndorphin_C|SetWasUsed _asplayer_start_ndorphin false)
        (goto _label))))
  (return (LocalVariables|GetSpawnToReturn)))