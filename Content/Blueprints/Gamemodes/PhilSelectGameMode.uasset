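; Game mode for a local multiplayer character select screen, which creates the menu widget and spawns local players up to the game instance's player count.
; Events activate players, cycle each controller's wrapping character selection, and confirm or back out.
; Player state is stored in NdorphinInstance containers and changes are mirrored to the widget.
; When all active players confirm and meet the minimum, LoadLevel can open the enum-named level.
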(event Custom|ChangeCharacterEvent
  (params (ControllerID :type Integer) (IsRight :type Boolean) (MoveSelection :type Boolean))
  (bind _cselection (CallFunction|MoveSelection ControllerID IsRight))
  (Default|ChangeCharacterEvent (Variables|Default|GetMenuWidget) ControllerID (Utilities|Text|ToText(String) (Utilities|GetClassDisplayName (Utilities|Array|Get(acopy) (Variables|/Game/Blueprints/NdorphinInstance.NdorphinInstance_C|GetCharacters (Variables|Default|GetGameInstance)) _cselection))) _cselection))

(event Custom|LoadLevel
  (bind _canstart (CallFunction|CheckifCanStart))
  (if _canstart
    (Game|OpenLevel(byName) (Utilities|String|StringToName (Utilities|String|EnumtoString (Variables|Default|GetSelectedLevel))))))

(event Custom|ActivatePlayerEvent
  (params (ControllerID :type Integer))
  (CallFunction|ActivatePlayer ControllerID))

(event Custom|BackEvent
  (params (ControllerID :type Integer) (PreviousState :type CharacterSelectState%20Enum :default "NewEnumerator0"))
  (CallFunction|UnConfirmSelection ControllerID PreviousState))

(event Custom|ConfirmSelectionEvent
  (params (ControllerID :type Integer))
  (CallFunction|ConfirmSelection ControllerID))

(event EventBeginPlay
  (bind _returnvalue (UserInterface|CreateWidget "/Game/Blueprints/Widgets]/PhilSelectWidget.PhilSelectWidget_C"))
  (bind _output_get (Variables|Default|SetMenuWidget _returnvalue))
  (UserInterface|Viewport|AddtoViewport _output_get 0)
  (bind _asndorphin_instance (Utilities|Casting|CastToNdorphinInstance (Game|GetGameInstance)))
  (Variables|Default|SetGameInstance _asndorphin_instance)
  (CallFunction|SpawnControllers))

(fn ConstructionScript)

(fn SpawnControllers
  (while (> (Variables|/Game/Blueprints/NdorphinInstance.NdorphinInstance_C|GetNumberOfPlayers (Variables|Default|GetGameInstance)) (LocalVariables|GetControllerID))
    (Class|GameplayStatics|CreatePlayer -1)
    (Math|Integer|IncrementInt (LocalVariables|GetControllerID))))

(fn ConfirmSelection
  (params (ControllerID :type Integer))
  (LocalVariables|SetController ControllerID)
  (Default|CreateorUpdatePlayerContainer (Variables|Default|GetGameInstance) (Utilities|Array|Get(acopy) (Variables|Default|GetCurrentSelections) (LocalVariables|GetController)) (LocalVariables|GetController) (LocalVariables|GetActive) (LocalVariables|GetConfirmed))
  (Default|ConfirmSelectionEvent (Variables|Default|GetMenuWidget) (LocalVariables|GetController))
  (bind _canstart (CallFunction|CheckifCanStart))
  (Default|ToggleStartBanner (Variables|Default|GetMenuWidget) _canstart))

(fn UnConfirmSelection
  (params (ControllerID :type Integer) (PreviousState :type CharacterSelectState%20Enum :default "NewEnumerator0"))
  (LocalVariables|SetController ControllerID)
  (LocalVariables|SetState PreviousState)
  (switch Utilities|FlowControl|Switch|SwitchonCharacterSelectState (LocalVariables|GetState)
    (:NewEnumerator1
      (LocalVariables|SetConfirmed false)
      (LocalVariables|SetActive false))
    (:NewEnumerator2
      (LocalVariables|SetConfirmed false)
      (LocalVariables|SetActive true)))
  (Default|CreateorUpdatePlayerContainer (Variables|Default|GetGameInstance) 0 (LocalVariables|GetController) (LocalVariables|GetActive) (LocalVariables|GetConfirmed))
  (Default|BackEvent (Variables|Default|GetMenuWidget) (LocalVariables|GetController) (LocalVariables|GetState)))

(fn MoveSelection
  (params (ControllerID :type Integer) (IsRight :type Boolean))
  (LocalVariables|SetRight IsRight)
  (LocalVariables|SetController ControllerID)
  (LocalVariables|SetAmountChars (Utilities|Array|Length (Variables|/Game/Blueprints/NdorphinInstance.NdorphinInstance_C|GetCharacters (Variables|Default|GetGameInstance))))
  (LocalVariables|SetSelection (Utilities|Array|Get(acopy) (Variables|Default|GetCurrentSelections) (LocalVariables|GetController)))
  (Utilities|FlowControl|Sequence
    (:then_0
      (if (LocalVariables|GetRight)
        (Math|Integer|IncrementInt (LocalVariables|GetSelection)
          (:%20%20
            (if (>= (LocalVariables|GetSelection) (LocalVariables|GetAmountChars))
              (LocalVariables|SetSelection 0))))
        (else
          (Math|Integer|DecrementInt (LocalVariables|GetSelection)
            (:%20%20
              (if (< (LocalVariables|GetSelection) 0)
                (LocalVariables|SetSelection (- (LocalVariables|GetAmountChars) 1))))))))
    (:then_1
      (Utilities|Array|SetArrayElem (Variables|Default|GetCurrentSelections) (LocalVariables|GetController) (LocalVariables|GetSelection))
      (return (LocalVariables|GetSelection)))))

(fn ActivatePlayer
  (params (ControllerID :type Integer))
  (LocalVariables|SetController ControllerID)
  (Default|CreateorUpdatePlayerContainer (Variables|Default|GetGameInstance) 0 (LocalVariables|GetController) true false)
  (Default|ActivatePlayerEvent (Variables|Default|GetMenuWidget) (LocalVariables|GetController) (Utilities|Text|ToText(String) (Utilities|GetClassDisplayName (Utilities|Array|Get(acopy) (Variables|/Game/Blueprints/NdorphinInstance.NdorphinInstance_C|GetCharacters (Variables|Default|GetGameInstance)))))))

(fn CheckifCanStart
  (bind _confirmedplayers (Default|GetConfirmedPlayers (Variables|Default|GetGameInstance)))
  (LocalVariables|SetConfirmed _confirmedplayers)
  (bind _activeplayers (Default|GetActivePlayers (Variables|Default|GetGameInstance)))
  (LocalVariables|SetActive _activeplayers)
  (Utilities|FlowControl|Sequence
    (:then_0
      (if (and (== (LocalVariables|GetConfirmed) (LocalVariables|GetActive)) (>= (LocalVariables|GetConfirmed) (Variables|Default|GetMinToStart)))
        (LocalVariables|SetIfCanStart true)))
    (:then_1
      (return (LocalVariables|GetIfCanStart)))))