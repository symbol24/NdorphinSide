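; Playable character Blueprint for The Pill that maps player input to the character's three actions.
; Fire, Ability and Super presses each call the matching use function on KillingMethode, Ability and Super respectively, so the action logic lives outside this graph.
; The construction script only calls its parent, and the BeginPlay, overlap and Tick events are disabled placeholders.
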(event EventBeginPlay
  (|CallParentFunction) ; This node is disabled and will not be called.\nDrag off pins to build functionality.
)

(event Collision|EventActorBeginOverlap
  (params (OtherActor :type Actor%20Object%20Reference))
  (|CallParentFunction OtherActor) ; This node is disabled and will not be called.\nDrag off pins to build functionality.
)

(event EventTick
  (params (DeltaSeconds :type Float%20%28single-precision%29))
  (|CallParentFunction DeltaSeconds) ; This node is disabled and will not be called.\nDrag off pins to build functionality.
)

(event Input|ActionEvents|InputActionAbility
  (params (Key :type Key%20Structure))
  (:Pressed
    (Default|UseAbility (Variables|Default|GetAbility))))

(event Input|ActionEvents|InputActionFire
  (params (Key :type Key%20Structure))
  (:Pressed
    (Default|UseKillingMethode (Variables|Default|GetKillingMethode))))

(event Input|ActionEvents|InputActionSuper
  (params (Key :type Key%20Structure))
  (:Pressed
    (Default|UseSuper (Variables|Default|GetSuper))))

(fn ConstructionScript
  (|CallParentFunction))