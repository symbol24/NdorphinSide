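; Dash ability component that launches a player's SideScrollerCharacter along the direction its firing point arrow faces.
; DashForward resolves the character from the EmptyController's player ID, then launches it if CanDash allows, stops movement after the dash duration and re-arms after a cooldown.
; Invincibility is set on every call, even during cooldown, and clears only when a successful dash's cooldown ends.
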(event Custom|DashForward
  (params (ControllerPawn :type Object%20Object%20Reference))
  (bind _asempty_controller (Utilities|Casting|CastToEmptyController ControllerPawn))
  (bind _returnvalue (Class|GameplayStatics|GetPlayerControllerID _asempty_controller))
  (bind _asside_scroller_character (Utilities|Casting|CastToSideScrollerCharacter (Game|GetPlayerCharacter _returnvalue)))
  (Variables|/Game/Blueprints/z_Depricated/SideScrollerCharacter.SideScrollerCharacter_C|SetIsInvincible _asside_scroller_character true)
  (if (Variables|Default|GetCanDash)
    (Variables|Default|SetCanDash false)
    (Character|LaunchCharacter (Game|GetPlayerCharacter _returnvalue) (* (Math|Vector|GetForwardVector (Variables|/Game/Blueprints/z_Depricated/SideScrollerCharacter.SideScrollerCharacter_C|GetFiringPointArrow _asside_scroller_character)) (Variables|Default|GetForceToPush)) false false)
    (Utilities|FlowControl|Delay (Variables|Default|GetDurationOfDash))
    (Components|Movement|StopMovementImmediately (Variables|/Script/Engine.Character|GetCharacterMovement _asside_scroller_character))
    (Utilities|FlowControl|Delay (Variables|Default|GetDashCoolDown))
    (Variables|Default|SetCanDash true)
    (Variables|/Game/Blueprints/z_Depricated/SideScrollerCharacter.SideScrollerCharacter_C|SetIsInvincible _asside_scroller_character false)))

(event EventBeginPlay)

(event EventTick
  (params (DeltaSeconds :type Float%20%28single-precision%29)))