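; Unicorn character ability that lays a timed trail of Magictrail actors.
; On BeginPlay it caches the owning player's controller ID and passes it to each spawned trail piece.
; UseAbility sets a flag that lets Tick, throttled by a Delay, spawn pieces at the owner's Arrow1-tagged arrow component.
; The CoolDown delay clears the flag, so it sets how long the trail lasts rather than blocking reuse.
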(event EventBeginPlay
  (bind _asndorphin_character_parent (Utilities|Casting|CastToNdorphinCharacter_Parent (Components|GetOwner)))
  (bind _asempty_controller (Utilities|Casting|CastToEmptyController (Pawn|GetController _asndorphin_character_parent)))
  (bind _returnvalue (Class|GameplayStatics|GetPlayerControllerID _asempty_controller))
  (Variables|Default|SetOwnerID _returnvalue))

(event EventTick
  (params (DeltaSeconds :type Float%20%28single-precision%29))
  (Utilities|FlowControl|Delay (Variables|Default|GetSpawnRate))
  (if (Variables|Default|GetStartCounting)
    (Game|SpawnActorfromClass "/Game/Blueprints/Objects/Magictrail.Magictrail_C" (Transformation|GetWorldTransform (Utilities|Array|Get(acopy) (Actor|GetComponentsbyTag (Components|GetOwner) "/Script/Engine.ArrowComponent" "Arrow1"))) "AdjustIfPossibleButAlwaysSpawn" 0 (Variables|Default|GetOwnerID) 0)
    (Utilities|FlowControl|Delay (Variables|Default|GetCoolDown))
    (Variables|Default|SetStartCounting false)))

(event EventUseAbility
  (Variables|Default|SetStartCounting true))