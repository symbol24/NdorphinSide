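; NdorphinInstance holds the player roster as an array of PlayerContainers tracking controller, character, active/confirmed state and score.
; Linear searches by ControllerID create, update, fetch or remove entries, and helpers count active and confirmed players.
; New players take the array length as PlayerID, which score updates use as an index, though removals never renumber it.
; Unconfirmed-player cleanup removes entries while iterating the same array.
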(fn CreateorUpdatePlayerContainer
  (params (CharacterID :type Integer) (ControllerID :type Integer) (IsActive :type Boolean) (IsConfirmed :type Boolean))
  (LocalVariables|SetCharID CharacterID)
  (LocalVariables|SetconID ControllerID)
  (LocalVariables|SetActive IsActive)
  (LocalVariables|SetConfirmed IsConfirmed)
  (bind (_array_element _array_index) (Utilities|Array|ForEachLoopwithBreak (Variables|Default|GetPlayerContainers) :!label _label)
    (:LoopBody
      (LocalVariables|Setindex _array_index)
      (bind _output_get (LocalVariables|SetPlayerContainer _array_element))
      (if (== (Utilities|Struct|BreakPlayerContainer _output_get) (LocalVariables|GetconID))
        (LocalVariables|SetFound true)
        (Utilities|Struct|SetmembersinPlayerContainer (LocalVariables|GetPlayerContainer) (LocalVariables|GetCharID) (LocalVariables|GetConfirmed) (LocalVariables|GetActive))
        (Utilities|Array|SetArrayElem (Variables|Default|GetPlayerContainers) (LocalVariables|Getindex) (LocalVariables|GetPlayerContainer))
        (goto _label Break)))
    (:Completed
      (if (LocalVariables|GetFound)
        _
        (else
          (bind _structout (Utilities|Struct|SetmembersinPlayerContainer (LocalVariables|GetPlayerContainer) (Utilities|Array|Length (Variables|Default|GetPlayerContainers)) (LocalVariables|GetCharID) (LocalVariables|GetconID) (LocalVariables|GetConfirmed) (LocalVariables|GetActive)))
          (Utilities|Array|Add (Variables|Default|GetPlayerContainers) _structout)))
      (return (LocalVariables|GetPlayerContainer)))))

(fn GetPlayerContianerfromControllerID
  (params (ControllerID :type Integer))
  (bind _array_element (Utilities|Array|ForEachLoopwithBreak (Variables|Default|GetPlayerContainers) :!label _label)
    (:LoopBody
      (bind _output_get (LocalVariables|SetIsFound (== (.ControllerID (Utilities|Struct|BreakPlayerContainer _array_element)) ControllerID)))
      (if _output_get
        (LocalVariables|SetContainer _array_element)
        (goto _label Break)))
    (:Completed
      (if (LocalVariables|GetIsFound)
        _
        (else
          (Development|PrintText (Utilities|Text|FormatText "Player Container not found from Controller ID {id}" ControllerID))))
      (return (LocalVariables|GetContainer)))))

(fn GetPlayerIDfromControllerID
  (params (ControllerID :type Integer))
  (bind _playercontainer (CallFunction|GetPlayerContianerfromControllerID ControllerID))
  (if (!= (.PlayerID (Utilities|Struct|BreakPlayerContainer _playercontainer)) -1)
    (LocalVariables|SetPlayerID (.PlayerID (Utilities|Struct|BreakPlayerContainer _playercontainer))))
  (return (LocalVariables|GetPlayerID)))

(fn UpdatePlayerScorefromID
  (params (PlayerID :type Integer) (Score :type Float%20%28single-precision%29))
  (LocalVariables|SetpID PlayerID)
  (LocalVariables|SetNewScore Score)
  (if (< (LocalVariables|GetpID) (Utilities|Array|Length (Variables|Default|GetPlayerContainers)))
    (Utilities|Struct|SetmembersinPlayerContainer (Utilities|Array|Get(acopy) (Variables|Default|GetPlayerContainers) (LocalVariables|GetpID)) (LocalVariables|GetNewScore))))

(fn RemovePlayerContainerfromControllerID
  (params (Controller :type Integer))
  (LocalVariables|SetControllerID Controller)
  (bind (_array_element _array_index) (Utilities|Array|ForEachLoopwithBreak (Variables|Default|GetPlayerContainers) :!label _label)
    (:LoopBody
      (LocalVariables|SetContainerID _array_index)
      (if (== (Utilities|Struct|BreakPlayerContainer _array_element) (LocalVariables|GetControllerID))
        (Utilities|Array|RemoveIndex (Variables|Default|GetPlayerContainers) (LocalVariables|GetContainerID))
        (goto _label Break)))))

(fn RemoveUnconfirmedPlayerContainers
  (for (_array_element _array_index) (Variables|Default|GetPlayerContainers)
    (LocalVariables|SetContainerId _array_index)
    (if (not (Utilities|Struct|BreakPlayerContainer _array_element))
      (Utilities|Array|RemoveIndex (Variables|Default|GetPlayerContainers) (LocalVariables|GetContainerId)))))

(fn GetConfirmedPlayers
  (for _array_element (Variables|Default|GetPlayerContainers)
    (if (Utilities|Struct|BreakPlayerContainer _array_element)
      (Math|Integer|IncrementInt (LocalVariables|GetConfirmed))))
  (return (LocalVariables|GetConfirmed)))

(fn GetActivePlayers
  (for _array_element (Variables|Default|GetPlayerContainers)
    (if (Utilities|Struct|BreakPlayerContainer _array_element)
      (Math|Integer|IncrementInt (LocalVariables|GetActive))))
  (return (LocalVariables|GetActive)))