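; Jump-through platform that ignores Pawn collision until a character enters its Trigger volume.
; Trigger overlap passes a DoOnce gate, waits briefly, then sets the Platform to block Pawns and raises IsHitting.
; End overlap resets the gate, restores pass-through and clears the flag, but does not cancel a pending delay.
; Collision changes apply to the whole Pawn channel, not just the overlapping character.
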(event OnComponentBeginOverlap(Trigger)
  (params (OverlappedComponent :type Primitive%20Component%20Object%20Reference) (OtherActor :type Actor%20Object%20Reference) (OtherComp :type Primitive%20Component%20Object%20Reference) (OtherBodyIndex :type Integer) (bFromSweep :type Boolean) (SweepResult :type Hit%20Result%20Structure%20%28by%20ref%29))
  (Utilities|Casting|CastToCharacter OtherActor)
  (Utilities|FlowControl|DoOnce false
    (:Completed
      (Utilities|FlowControl|Delay 0.2)
      (Collision|SetCollisionResponsetoChannel (Variables|Default|GetPlatform) "ECC_Pawn" "ECR_Block")
      (Variables|Default|SetIsHitting true))))

(event OnComponentEndOverlap(Trigger)
  (params (OverlappedComponent :type Primitive%20Component%20Object%20Reference) (OtherActor :type Actor%20Object%20Reference) (OtherComp :type Primitive%20Component%20Object%20Reference) (OtherBodyIndex :type Integer))
  (Utilities|Casting|CastToCharacter OtherActor)
  (CallFunction|Reset)
  (Collision|SetCollisionResponsetoChannel (Variables|Default|GetPlatform) "ECC_Pawn" "ECR_Ignore")
  (Variables|Default|SetIsHitting false))

(event Custom|Reset
  (Utilities|FlowControl|DoOnce false) ; enters at Reset
)

(event EventBeginPlay
  (Collision|SetCollisionResponsetoChannel (Variables|Default|GetPlatform) "ECC_Pawn" "ECR_Ignore"))

(fn ConstructionScript)